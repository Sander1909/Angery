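; Game mode Blueprint that handles next-wave announcements and the victory transition in a wave-based game.
; On BeginPlay it creates the NextWave widget, adds it to the viewport hidden and keeps a reference.
; NextWaveAnnouncement briefly shows that widget, then hides it again.
; Despite its name, ShowVictoryHUD displays no widget and instead opens the Victory level after a short delay.
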(event `self.ShowVictoryHUD`
  (`KismetSystemLibrary.Delay` 2.0)
  (`GameplayStatics.OpenLevel` "Victory"))

(event `self.ReceiveBeginPlay`
  ;[1 1 1] Display Next Wave Text
  (bind _returnvalue (`|CreateWidget` "/Game/HUDAssets/NextWave.NextWave_C"))
  (bind _output_get (set `self.NextWaveReference` _returnvalue))
  (`UserWidget.AddToViewport` _output_get 0)
  (`Widget.SetVisibility` _output_get "Hidden"))

(event `self.NextWaveAnnouncement`
  ;[1 1 1] Display Next Wave Text
  (`Widget.SetVisibility` (stale `self.ReceiveBeginPlay` _output_get) "Visible")
  (`KismetSystemLibrary.Delay` 1.5)
  (`Widget.SetVisibility` (stale `self.ReceiveBeginPlay` _output_get) "Hidden"))

(fn `UserConstructionScript`)