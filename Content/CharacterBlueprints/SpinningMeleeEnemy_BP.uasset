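; Spinning melee enemy Blueprint that keeps its overhead health bar and movement state up to date.
; Each tick it casts its widget component to AI_Health and sets the progress bar to current health over max health.
; It also sets IsMoving from whether its velocity is nonzero, while the construction script is empty.
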(event `self.ReceiveTick`
  (params (DeltaSeconds :type "Float (single-precision)"))
  ;[1 1 1] Enemy Health Bar
  (bind _asai_health (cast `/Game/HUDAssets/AI_Health` (`WidgetComponent.GetUserWidgetObject` (`self.Widget`))))
  (`ProgressBar.SetPercent` (`/Game/HUDAssets/AI_Health.ProgressBar_240` _asai_health) (/ (`KismetMathLibrary.Conv_IntToDouble` (`self.Health`)) (`self.MaxHealth`)))
  (set `self.bIsMoving` (> (`KismetMathLibrary.VSize` (`self.GetVelocity` self)) 0.0)))

(fn `UserConstructionScript`)